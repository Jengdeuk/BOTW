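; BP_BatteryBeam is a beam attack from a BP_Battery that reaches toward a target location and explodes.
; Each tick it eases the beam end from the battery's head to the target over one second, updating the effect and sweeping its collision along.
; An overlap with a Link or Teba tagged actor, or the timer expiring, spawns an enlarged BP_Explosion at the target; the beam destroys itself a second later.
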(event `self.ReceiveBeginPlay`
  (add `PrimitiveComponent.OnComponentBeginOverlap` (`self.Collision`) (delegate `OnHit`)))

(event `OnHit`
  (params (OverlappedComponent :type "PrimitiveComponent Object Reference") (OtherActor :type "Actor Object Reference") (OtherComp :type "PrimitiveComponent Object Reference") (OtherBodyIndex :type Integer) (bFromSweep :type Boolean) (SweepResult :type "HitResult Structure (by ref)"))
  ; 충돌처리
  (if (or (`self.ActorHasTag` OtherActor "Link") (`self.ActorHasTag` OtherActor "Teba"))
    (`self.OnExplosion`)))

(event `OnExplosion`
  ; 폭발하기
  (`|SpawnActorFromClass` "/Game/Blueprints/Effect/BP_Explosion.BP_Explosion_C" (`KismetMathLibrary.MakeTransform` (`self.TargetLoc`) (struct) (6.0 6.0 6.0)) "Undefined" "MultiplyWithRoot" null null)
  (set `self.HasExplosion` true)
  (set `self.LifeTime` 1.0))

(event `self.ReceiveTick`
  (params (DeltaSeconds :type "Float (single-precision)"))
  (bind _output_get (set `self.LifeTime` (+ (`self.LifeTime`) DeltaSeconds)))
  (if (and (>= _output_get 1.0) (not (`self.HasExplosion`)))
    (`self.OnExplosion`)
    (elif (>= _output_get 2.0)
      (`self.K2_DestroyActor`)
      (else
        (`|ExecutionSequence`
          (:`then_0`
            ; 빔 이동
            (if true
              (bind _asbp_battery (cast `/Game/Blueprints/Battery/BP_Battery` (`self.OwnerBattery`)))
              (set `self.StartLoc` (`SceneComponent.K2_GetComponentLocation` (`/Game/Blueprints/Battery/BP_Battery.HeadCollision` _asbp_battery)))
              (set `self.CurrentLoc` (`|EaseFunction` "EaseIn" (`KismetMathLibrary.FClamp` _output_get) (`self.StartLoc`) (`self.TargetLoc`) 3.0))
              ; 빔 그리기
              (`NiagaraComponent.SetVariableVec3` (`self.BeamEffect`) "Beam Start" (`self.StartLoc`))
              (`NiagaraComponent.SetVariableVec3` (`self.BeamEffect`) "Beam End" (`self.CurrentLoc`))))
          (:`then_1`
            (`SceneComponent.K2_SetWorldLocation` (`self.Collision`) (`self.CurrentLoc`) true false)))))))

(fn `UserConstructionScript`)