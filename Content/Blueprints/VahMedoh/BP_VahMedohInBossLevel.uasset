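; Vah Medoh actor for the boss level, circling a center point and providing updraft zones for BP_Link.
; Each Tick steps the orbit angle in the negative direction, sets position from radius and height, and yaws along the center-to-slightly-ahead-point direction.
; Seven box triggers feed OnSetUpdraft, toggling Link's IsInUpdraft on begin and end overlap, without counting overlapping boxes.
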(event `OnSetUpdraft`
  (params (OtherActor :type "Actor Object Reference") (IsInUpdraft :type Boolean))
  ; 상승 기류
  (bind _asbp_link (cast `/Game/Blueprints/Link/BP_Link` OtherActor))
  (set `/Game/Blueprints/Link/BP_Link.IsInUpdraft` IsInUpdraft _asbp_link))

(event `self.Box1.OnComponentBeginOverlap`
  (params (OverlappedComponent :type "PrimitiveComponent Object Reference") (OtherActor :type "Actor Object Reference") (OtherComp :type "PrimitiveComponent Object Reference") (OtherBodyIndex :type Integer) (bFromSweep :type Boolean) (SweepResult :type "HitResult Structure (by ref)"))
  ; 상승 기류
  (`self.OnSetUpdraft` OtherActor true))

(event `self.Box.OnComponentBeginOverlap`
  (params (OverlappedComponent :type "PrimitiveComponent Object Reference") (OtherActor :type "Actor Object Reference") (OtherComp :type "PrimitiveComponent Object Reference") (OtherBodyIndex :type Integer) (bFromSweep :type Boolean) (SweepResult :type "HitResult Structure (by ref)"))
  ; 상승 기류
  (`self.OnSetUpdraft` OtherActor true))

(event `self.Box4.OnComponentBeginOverlap`
  (params (OverlappedComponent :type "PrimitiveComponent Object Reference") (OtherActor :type "Actor Object Reference") (OtherComp :type "PrimitiveComponent Object Reference") (OtherBodyIndex :type Integer) (bFromSweep :type Boolean) (SweepResult :type "HitResult Structure (by ref)"))
  ; 상승 기류
  (`self.OnSetUpdraft` OtherActor true))

(event `self.ReceiveTick`
  (params (DeltaSeconds :type "Float (single-precision)"))
  (bind (_returnvalue_roll _returnvalue_pitch) (`KismetMathLibrary.BreakRotator` (`self.K2_GetActorRotation`)))
  (bind (_orbitcenter_x _orbitcenter_y _orbitcenter_z) (`KismetMathLibrary.BreakVector` (`self.OrbitCenter`)))
  (bind (_orbitcenter_x_2 _orbitcenter_y_2 _orbitcenter_z_2) (`KismetMathLibrary.BreakVector` (`self.OrbitCenter`)))
  (bind _returnvalue (+ (`self.CurrentAngleRad`) (* (`KismetMathLibrary.DegreesToRadians` (`self.AngularSpeedDeg`)) 0.05 -1.0)))
  (bind (_returnvalue_roll_2 _returnvalue_pitch_2 _returnvalue_yaw) (`KismetMathLibrary.BreakRotator` (`KismetMathLibrary.FindLookAtRotation` (`KismetMathLibrary.MakeVector` _orbitcenter_x _orbitcenter_y _orbitcenter_z) (`KismetMathLibrary.MakeVector` (+ (* (`self.OrbitRadius`) (`KismetMathLibrary.Cos` _returnvalue)) _orbitcenter_x_2) (+ (* (`self.OrbitRadius`) (`KismetMathLibrary.Sin` _returnvalue)) _orbitcenter_y_2) (+ (`self.OrbitHeight`) _orbitcenter_z_2)))))
  ; SetCurrentAngle
  (set `self.CurrentAngleRad` (+ (`self.CurrentAngleRad`) (* (`KismetMathLibrary.DegreesToRadians` (`self.AngularSpeedDeg`)) DeltaSeconds -1.0)))
  ; Movement
  (`self.K2_SetActorLocation` (`KismetMathLibrary.MakeVector` (+ (* (`self.OrbitRadius`) (`KismetMathLibrary.Cos` (`self.CurrentAngleRad`))) _orbitcenter_x) (+ (* (`self.OrbitRadius`) (`KismetMathLibrary.Sin` (`self.CurrentAngleRad`))) _orbitcenter_y) (+ (`self.OrbitHeight`) _orbitcenter_z)))
  (`self.K2_SetActorRotation` (`KismetMathLibrary.MakeRotator` _returnvalue_roll _returnvalue_pitch _returnvalue_yaw)))

(event `self.Box1.OnComponentEndOverlap`
  (params (OverlappedComponent :type "PrimitiveComponent Object Reference") (OtherActor :type "Actor Object Reference") (OtherComp :type "PrimitiveComponent Object Reference") (OtherBodyIndex :type Integer))
  ; 상승 기류
  (`self.OnSetUpdraft` OtherActor))

(event `self.Box.OnComponentEndOverlap`
  (params (OverlappedComponent :type "PrimitiveComponent Object Reference") (OtherActor :type "Actor Object Reference") (OtherComp :type "PrimitiveComponent Object Reference") (OtherBodyIndex :type Integer))
  ; 상승 기류
  (`self.OnSetUpdraft` OtherActor))

(event `self.Box4.OnComponentEndOverlap`
  (params (OverlappedComponent :type "PrimitiveComponent Object Reference") (OtherActor :type "Actor Object Reference") (OtherComp :type "PrimitiveComponent Object Reference") (OtherBodyIndex :type Integer))
  ; 상승 기류
  (`self.OnSetUpdraft` OtherActor))

(event `self.Box3.OnComponentBeginOverlap`
  (params (OverlappedComponent :type "PrimitiveComponent Object Reference") (OtherActor :type "Actor Object Reference") (OtherComp :type "PrimitiveComponent Object Reference") (OtherBodyIndex :type Integer) (bFromSweep :type Boolean) (SweepResult :type "HitResult Structure (by ref)"))
  ; 상승 기류
  (`self.OnSetUpdraft` OtherActor true))

(event `self.Box5.OnComponentBeginOverlap`
  (params (OverlappedComponent :type "PrimitiveComponent Object Reference") (OtherActor :type "Actor Object Reference") (OtherComp :type "PrimitiveComponent Object Reference") (OtherBodyIndex :type Integer) (bFromSweep :type Boolean) (SweepResult :type "HitResult Structure (by ref)"))
  ; 상승 기류
  (`self.OnSetUpdraft` OtherActor true))

(event `self.Box2.OnComponentBeginOverlap`
  (params (OverlappedComponent :type "PrimitiveComponent Object Reference") (OtherActor :type "Actor Object Reference") (OtherComp :type "PrimitiveComponent Object Reference") (OtherBodyIndex :type Integer) (bFromSweep :type Boolean) (SweepResult :type "HitResult Structure (by ref)"))
  ; 상승 기류
  (`self.OnSetUpdraft` OtherActor true))

(event `self.Box3.OnComponentEndOverlap`
  (params (OverlappedComponent :type "PrimitiveComponent Object Reference") (OtherActor :type "Actor Object Reference") (OtherComp :type "PrimitiveComponent Object Reference") (OtherBodyIndex :type Integer))
  ; 상승 기류
  (`self.OnSetUpdraft` OtherActor))

(event `self.Box5.OnComponentEndOverlap`
  (params (OverlappedComponent :type "PrimitiveComponent Object Reference") (OtherActor :type "Actor Object Reference") (OtherComp :type "PrimitiveComponent Object Reference") (OtherBodyIndex :type Integer))
  ; 상승 기류
  (`self.OnSetUpdraft` OtherActor))

(event `self.Box2.OnComponentEndOverlap`
  (params (OverlappedComponent :type "PrimitiveComponent Object Reference") (OtherActor :type "Actor Object Reference") (OtherComp :type "PrimitiveComponent Object Reference") (OtherBodyIndex :type Integer))
  ; 상승 기류
  (`self.OnSetUpdraft` OtherActor))

(event `self.Box6.OnComponentBeginOverlap`
  (params (OverlappedComponent :type "PrimitiveComponent Object Reference") (OtherActor :type "Actor Object Reference") (OtherComp :type "PrimitiveComponent Object Reference") (OtherBodyIndex :type Integer) (bFromSweep :type Boolean) (SweepResult :type "HitResult Structure (by ref)"))
  ; 상승 기류
  (`self.OnSetUpdraft` OtherActor true))

(event `self.Box6.OnComponentEndOverlap`
  (params (OverlappedComponent :type "PrimitiveComponent Object Reference") (OtherActor :type "Actor Object Reference") (OtherComp :type "PrimitiveComponent Object Reference") (OtherBodyIndex :type Integer))
  ; 상승 기류
  (`self.OnSetUpdraft` OtherActor))

(fn `UserConstructionScript`)