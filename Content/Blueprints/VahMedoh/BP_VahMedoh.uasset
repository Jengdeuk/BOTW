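; BP_VahMedoh is the Vah Medoh actor, which circles a center point at a fixed radius and height once activated.
; It starts hidden with collision and tick off, and SetActorActivate toggles all three together.
; Each Tick decreases the orbit angle by angular speed and delta time, then places the actor using sine and cosine.
; Yaw points from the orbit center toward a slightly look-ahead orbit position, keeping roll and pitch unchanged.
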(event `self.ReceiveBeginPlay`
  ; Init
  (`self.SetActorActivate` false))

(event `SetActorActivate`
  (params (IsActive :type Boolean))
  ; Activation
  (`self.SetActorHiddenInGame` (not IsActive))
  (`self.SetActorEnableCollision` IsActive)
  (`self.SetActorTickEnabled` IsActive))

(event `self.ReceiveTick`
  (params (DeltaSeconds :type "Float (single-precision)"))
  (bind (_returnvalue_roll _returnvalue_pitch) (`KismetMathLibrary.BreakRotator` (`self.K2_GetActorRotation`)))
  (bind (_orbitcenter_x _orbitcenter_y _orbitcenter_z) (`KismetMathLibrary.BreakVector` (`self.OrbitCenter`)))
  (bind (_orbitcenter_x_2 _orbitcenter_y_2 _orbitcenter_z_2) (`KismetMathLibrary.BreakVector` (`self.OrbitCenter`)))
  (bind _returnvalue (+ (`self.CurrentAngleRad`) (* (`KismetMathLibrary.DegreesToRadians` (`self.AngularSpeedDeg`)) 0.05 -1.0)))
  (bind (_returnvalue_roll_2 _returnvalue_pitch_2 _returnvalue_yaw) (`KismetMathLibrary.BreakRotator` (`KismetMathLibrary.FindLookAtRotation` (`KismetMathLibrary.MakeVector` _orbitcenter_x _orbitcenter_y _orbitcenter_z) (`KismetMathLibrary.MakeVector` (+ (* (`self.OrbitRadius`) (`KismetMathLibrary.Cos` _returnvalue)) _orbitcenter_x_2) (+ (* (`self.OrbitRadius`) (`KismetMathLibrary.Sin` _returnvalue)) _orbitcenter_y_2) (+ (`self.OrbitHeight`) _orbitcenter_z_2)))))
  ; SetCurrentAngle
  (set `self.CurrentAngleRad` (+ (`self.CurrentAngleRad`) (* (`KismetMathLibrary.DegreesToRadians` (`self.AngularSpeedDeg`)) DeltaSeconds -1.0)))
  ; Movement
  (`self.K2_SetActorLocation` (`KismetMathLibrary.MakeVector` (+ (* (`self.OrbitRadius`) (`KismetMathLibrary.Cos` (`self.CurrentAngleRad`))) _orbitcenter_x) (+ (* (`self.OrbitRadius`) (`KismetMathLibrary.Sin` (`self.CurrentAngleRad`))) _orbitcenter_y) (+ (`self.OrbitHeight`) _orbitcenter_z)))
  (`self.K2_SetActorRotation` (`KismetMathLibrary.MakeRotator` _returnvalue_roll _returnvalue_pitch _returnvalue_yaw)))

(fn `UserConstructionScript`)