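; BP_Battery is a destructible battery in the Vah Medoh content that breaks after repeated damage.
; Its OnDamaged event increments a hit counter and triggers the break only when the count equals three.
; Breaking swaps the skeletal mesh to a broken version, disables head collision, attaches smoke and spark emitters to the body, and spawns a scaled-up BP_Explosion at the head's location.
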(event `OnDamaged`
  (bind _headcollision (`self.HeadCollision`))
  (bind _bodycollision (`self.BodyCollision`))
  (bind _result (`/Engine/EditorBlueprintResources/StandardMacros.IncrementInt` (`self.DamagedCount`))
    (:`  `
      (if (== _result 3)
        (set `SkeletalMeshComponent.SkeletalMeshAsset` "/Game/Assets/Battery/BatteryBroken/BatteryBroken.BatteryBroken" (`self.SkeletalMesh`))
        (`GameplayStatics.SpawnEmitterAttached` "/Game/Realistic_Starter_VFX_Pack_Vol2/Particles/Smoke/P_Smoke_B.P_Smoke_B" _bodycollision "None" (0.0 0.0 0.0) (struct) (15.0 15.0 15.0))
        (`PrimitiveComponent.SetCollisionEnabled` _headcollision "NoCollision")
        (`GameplayStatics.SpawnEmitterAttached` "/Game/Realistic_Starter_VFX_Pack_Vol2/Particles/Sparks/P_Sparks_C.P_Sparks_C" _bodycollision "None" (0.0 0.0 0.0) (struct) (15.0 15.0 15.0))
        (`|SpawnActorFromClass` "/Game/Blueprints/Effect/BP_Explosion.BP_Explosion_C" (`KismetMathLibrary.MakeTransform` (`SceneComponent.K2_GetComponentLocation` _headcollision) (struct) (6.0 6.0 6.0)) "Undefined" "MultiplyWithRoot" null null)))))

(fn `UserConstructionScript`)