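; Animation notify that fires Ganon's beam shot when it triggers during an animation.
; It spawns a BP_GanonBullet2 at the mesh's Fire socket and sets its projectile velocity along Ganon's FireDir at the projectile's initial speed.
; It then increments Ganon's attack action count, and does nothing if the mesh owner is not BP_Ganon.
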(fn `Received_Notify`
  (params (MeshComp :type "SkeletalMeshComponent Object Reference") (Animation :type "AnimSequenceBase Object Reference") (EventReference :type "AnimNotifyEventReference Structure (by ref)"))
  (returns (ReturnValue :type Boolean))
  (bind _asbp_ganon (cast `/Game/Blueprints/Ganon/BP_Ganon` (`ActorComponent.GetOwner` MeshComp))
    (:`then`
      (bind _returnvalue (`|SpawnActorFromClass` "/Game/Blueprints/Projectile/BP_GanonBullet2.BP_GanonBullet2_C" (`KismetMathLibrary.MakeTransform` (`SceneComponent.GetSocketLocation` MeshComp "Fire")) "Undefined" "MultiplyWithRoot" null null))
      (bind _projectilemovement (`/Game/Blueprints/Projectile/BP_GanonBullet2.ProjectileMovement` _returnvalue))
      (bind _initialspeed (`ProjectileMovementComponent.InitialSpeed` _projectilemovement))
      (set `MovementComponent.Velocity` (* (`/Game/Blueprints/Ganon/BP_Ganon.FireDir` _asbp_ganon) (`KismetMathLibrary.MakeVector` _initialspeed _initialspeed _initialspeed)) _projectilemovement)
      (`/Game/Blueprints/Ganon/BP_Ganon.AddAttackActionCount` _asbp_ganon))
    (:`CastFailed`
      _))
  (return false))