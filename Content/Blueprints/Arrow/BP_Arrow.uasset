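; BP_Arrow is a projectile that explodes on impact and damages batteries.
; On a collision hit, it calls OnDamaged on a BP_Battery if the hit component is tagged BatteryCollision, then spawns a scaled-up BP_Explosion and destroys itself.
; Each tick it offsets global time dilation to keep normal speed during time scaling, aligns its rotation to velocity and self-destructs after a fixed lifetime.
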(event `self.ReceiveBeginPlay`
  (add `PrimitiveComponent.OnComponentHit` (`self.Collision`) (delegate `OnHit`)))

(event `OnHit`
  (params (HitComponent :type "PrimitiveComponent Object Reference") (OtherActor :type "Actor Object Reference") (OtherComp :type "PrimitiveComponent Object Reference") (NormalImpulse :type "Vector Structure") (Hit :type "HitResult Structure (by ref)"))
  (`|ExecutionSequence`
    (:`then_0`
      (if (`ActorComponent.ComponentHasTag` OtherComp "BatteryCollision")
        (bind _asbp_battery (cast `/Game/Blueprints/VahMedoh/BP_Battery` OtherActor))
        (`/Game/Blueprints/VahMedoh/BP_Battery.OnDamaged` _asbp_battery)))
    (:`then_1`
      (`|SpawnActorFromClass` "/Game/Blueprints/Effect/BP_Explosion.BP_Explosion_C" (`KismetMathLibrary.MakeTransform` Hit_Location (struct) (4.0 4.0 4.0)) "Undefined" "MultiplyWithRoot" null null)
      (`self.K2_DestroyActor`))))

(event `self.ReceiveTick`
  (params (DeltaSeconds :type "Float (single-precision)"))
  (set `self.CustomTimeDilation` (/ 1.0 (`GameplayStatics.GetGlobalTimeDilation`)))
  (`self.K2_SetActorRotation` (`KismetMathLibrary.MakeRotFromX` (`KismetMathLibrary.Normal` (`MovementComponent.Velocity` (`self.ProjectileMovement`)))))
  (bind _output_get (set `self.LifeTime` (+ (`self.LifeTime`) DeltaSeconds)))
  (if (>= _output_get 30.0)
    (`self.K2_DestroyActor`)))

(fn `UserConstructionScript`)