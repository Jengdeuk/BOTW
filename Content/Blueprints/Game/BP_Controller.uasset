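; BP_Controller is the player controller that drives the title screen, story dialogue and handoff from cinematics to gameplay.
; Enhanced Input actions toggle and confirm choices on the HUD or advance dialogue, and keep working while the title pauses the game.
; Chapter, scene and step counters index dialogue, with BP_CinematicManager playing the next sequence when a scene runs out.
; The final choice scene unloads the cinematic level, possesses a gliding Link and activates Vah Medoh.
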(event `self.ReceiveBeginPlay`
  (`|ExecutionSequence`
    (:`then_0`
      ; 입력 초기화
      (`EnhancedInputSubsystemInterface.AddMappingContext` (subsystem `EnhancedInputLocalPlayerSubsystem`) "/Game/Input/IMC_Game.IMC_Game" 0 (struct))
      (set `self.bShouldPerformFullTickWhenPaused` true)
      (`self.SetTickableWhenPaused` true))
    (:`then_1`
      ; HUD 초기화
      (`UserWidget.AddToViewport` (`self.HUD`) 0)
      (`self.UpdateShowDialogUI` (`self.IsShowDialog`)))
    (:`then_2`
      ; CinematicManager 초기화
      (bind _outactors (`GameplayStatics.GetAllActorsOfClass` "/Game/Blueprints/Cinematic/BP_CinematicManager.BP_CinematicManager_C"))
      (set `self.CinematicManager` (`|GetArrayItem` _outactors)))))

(event `UpdateShowDialogUI`
  (params (IsShow :type Boolean))
  (bind _dialogpanel (`/Game/Blueprints/UI/WBP_HUD.DialogPanel` (`self.HUD`)))
  ; 대화 보이기
  (bind _output_get (set `self.IsShowDialog` IsShow))
  (if _output_get
    (`Widget.SetVisibility` _dialogpanel "Visible")
    (else
      (`Widget.SetVisibility` _dialogpanel "Hidden"))))

(event `ProcessNextDialog`
  (bind _hud (`self.HUD`))
  (bind _hud_2 (`self.HUD`))
  (bind _hud_3 (`self.HUD`))
  ; 다음 대화로 넘기기
  (if (== (`self.SceneStep`) 4)
    (if (== (`self.DialogStep`) 0)
      (`/Game/Blueprints/UI/WBP_HUD.SetDialogByIndex` _hud_3 0 3 0)
      (`Widget.SetVisibility` (`/Game/Blueprints/UI/WBP_HUD.NextButtonImg` _hud_3) "Hidden")
      (if (`/Game/Blueprints/UI/WBP_HUD.IsShowDialogOptions` _hud)
        (`/Game/Blueprints/UI/WBP_HUD.ProcessChoiseOptionInDialogFirst` _hud)
        (`/Game/Blueprints/UI/WBP_HUD.SetDialogByIndex` _hud_2 0 3 1)
        (`Widget.SetVisibility` (`/Game/Blueprints/UI/WBP_HUD.NextButtonImg` _hud_2) "Visible")
        (set `self.DialogStep` 1))
      (else
        (`self.UpdateShowDialogUI` false)
        (`self.StartGame`)))
    (else
      (bind _result (`/Engine/EditorBlueprintResources/StandardMacros.IncrementInt` (`self.DialogStep`))
        (:`  `
          (bind _inrange (`/Game/Blueprints/UI/WBP_HUD.SetDialogByIndex` (`self.HUD`) (- (`self.ChapterStep`) 1) (- (`self.SceneStep`) 1) (- _result 1)))
          (if (not _inrange)
            (set `self.DialogStep` 0)
            (`/Engine/EditorBlueprintResources/StandardMacros.IncrementInt` (`self.SceneStep`)
              (:`  `
                (`self.ProcessNextDialog`)
                (`self.UpdateShowDialogUI` false)
                (`/Game/Blueprints/Cinematic/BP_CinematicManager.PlayNextSquence` (`self.CinematicManager`))))))))))

(event `EnhancedInput|/Game/Input/Actions/IA_ShowTitle`
  (params (ActionValue :type Boolean) (ElapsedSeconds :type "Float (double-precision)") (TriggeredSeconds :type "Float (double-precision)") (InputAction :type "InputAction Object Reference" :default "/Game/Input/Actions/IA_ShowTitle.IA_ShowTitle"))
  ; 타이틀 보이기
  (:`Started`
    (`self.ShowTitle`)))

(event `ShowTitle`
  ; 타이틀 보이기
  (`self.PauseGame` true)
  (`Widget.SetVisibility` (`/Game/Blueprints/UI/WBP_HUD.TitlePanel` (`self.HUD`)) "Visible"))

(event `EnhancedInput|/Game/Input/Actions/IA_SelectOption`
  (params (ActionValue :type Boolean) (ElapsedSeconds :type "Float (double-precision)") (TriggeredSeconds :type "Float (double-precision)") (InputAction :type "InputAction Object Reference" :default "/Game/Input/Actions/IA_SelectOption.IA_SelectOption"))
  (bind _hud (`self.HUD`))
  (:`Started`
    (if (`Widget.IsVisible` (`/Game/Blueprints/UI/WBP_HUD.TitlePanel` _hud))
      ; Space 입력 - Title
      (`/Game/Blueprints/UI/WBP_HUD.ProcessChoiseOptionInTitle` _hud)
      (else
        ; Space 입력 - Dialog
        (if (`self.IsShowDialog`)
          (`self.ProcessNextDialog`))))))

(event `EnhancedInput|/Game/Input/Actions/IA_ChoiseToggle`
  (params (ActionValue :type Boolean) (ElapsedSeconds :type "Float (double-precision)") (TriggeredSeconds :type "Float (double-precision)") (InputAction :type "InputAction Object Reference" :default "/Game/Input/Actions/IA_ChoiseToggle.IA_ChoiseToggle"))
  ; UI 선택 토글 입력
  (:`Started`
    (`/Game/Blueprints/UI/WBP_HUD.ChoiseToggle` (`self.HUD`))))

(event `ShowDialogOptions`
  (params (IsShow :type Boolean))
  ; Dialog 선택지 보이기
  (`/Game/Blueprints/UI/WBP_HUD.ShowDialogOptions` (`self.HUD`) IsShow))

(event `PauseGame`
  (params (IsPause :type Boolean))
  ; 게임 상태 관리
  (`GameplayStatics.SetGamePaused` IsPause))

(event `QuitGame`
  ; 게임 상태 관리
  (`KismetSystemLibrary.QuitGame` self "Quit"))

(event `StartGame`
  ; 게임 상태 관리
  (`|ExecutionSequence`
    (:`then_0`
      (`GameplayStatics.UnloadStreamLevel` "Sky_SealBreak_Cinematic"))
    (:`then_1`
      (bind _outactors (`GameplayStatics.GetAllActorsWithTag` "Link"))
      (bind _asbp_link (cast `/Game/Blueprints/Link/BP_Link` (`|GetArrayItem` _outactors)))
      (`self.Possess` _asbp_link)
      (`/Game/Blueprints/Link/BP_Link.SetActorActivate` _asbp_link true)
      (`/Game/Blueprints/Link/BP_Link.Glide` _asbp_link))
    (:`then_2`
      (bind _outactors_2 (`GameplayStatics.GetAllActorsWithTag` "VahMedoh"))
      (bind _asbp_vah_medoh (cast `/Game/Blueprints/VahMedoh/BP_VahMedoh` (`|GetArrayItem` _outactors_2)))
      (`/Game/Blueprints/VahMedoh/BP_VahMedoh.SetActorActivate` _asbp_vah_medoh true))))

(fn `UserConstructionScript`)