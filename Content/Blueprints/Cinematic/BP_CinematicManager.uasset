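; BP_CinematicManager steps through an ordered list of cinematic scenes, each with a sequence player.
; On BeginPlay it binds every player's finished event, starts the first sequence and pauses the game.
; PlayNextSquence stops the previous sequence and plays the next via a step counter.
; A finished sequence only switches the player's view to Camera; it does not advance the step.
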(event `self.ReceiveBeginPlay`
  ; Init
  (for _array_element (`self.Scenes`)
    (add `MovieSceneSequencePlayer.OnFinished` (`LevelSequenceActor.SequencePlayer` _array_element) (delegate `OnFinishedScene`)))
  (`self.PlayNextSquence`)
  (`GameplayStatics.SetGamePaused` true))

(event `OnFinishedScene`
  ; Init
  (`PlayerController.SetViewTargetWithBlend` (`GameplayStatics.GetPlayerController` 0) (`self.Camera`) 0.0 "VTBlend_Linear" 0.0 false))

(event `PlayNextSquence`
  (bind _returnvalue (- (`self.SceneStep`) 1))
  ; 다음 시퀀스 재생
  (`|ExecutionSequence`
    (:`then_0`
      (if (>= _returnvalue 0)
        (`MovieSceneSequencePlayer.Stop` (`LevelSequenceActor.SequencePlayer` (`|GetArrayItem` (`self.Scenes`) _returnvalue)))))
    (:`then_1`
      (bind _result (`/Engine/EditorBlueprintResources/StandardMacros.IncrementInt` (`self.SceneStep`))
        (:`  `
          (bind _returnvalue_2 (- _result 1))
          (if (< _returnvalue_2 (`KismetArrayLibrary.Array_Length` (`self.Scenes`)))
            (`MovieSceneSequencePlayer.Play` (`LevelSequenceActor.SequencePlayer` (`|GetArrayItem` (`self.Scenes`) _returnvalue_2)))))))))

(fn `UserConstructionScript`)