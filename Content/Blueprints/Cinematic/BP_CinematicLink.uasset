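; BP_CinematicLink is a cinematic actor that slowly rises and falls once its HasStartFlying flag is set.
; Tick accumulates RunningTime and adds a small, scaled sine of it to the actor's current Z, leaving X and Y unchanged.
; The offset is added per frame without delta-time scaling, so the travel height depends on frame rate.
; Nothing in this Blueprint sets the flag, and the construction script is empty.
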(event `self.ReceiveTick`
  (params (DeltaSeconds :type "Float (single-precision)"))
  (bind (_returnvalue_x _returnvalue_y _returnvalue_z) (`KismetMathLibrary.BreakVector` (`self.K2_GetActorLocation`)))
  (if (`self.HasStartFlying`)
    (bind _output_get (set `self.RunningTime` (+ (`self.RunningTime`) DeltaSeconds)))
    (`self.K2_SetActorLocation` (`KismetMathLibrary.MakeVector` _returnvalue_x _returnvalue_y (+ _returnvalue_z (* (`KismetMathLibrary.Sin` (* _output_get 0.3)) 0.5))))))

(fn `UserConstructionScript`)