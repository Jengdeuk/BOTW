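; BP_CinematicController drives dialog progression between cinematic scenes through player input.
; On BeginPlay it adds the game input mapping, shows the HUD and finds the BP_CinematicManager in the level.
; IA_Space steps through dialog images stored by chapter and scene in the HUD.
; When a scene's dialogs run out, it hides the panel, advances the scene and has the manager play the next sequence.
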(event `self.ReceiveBeginPlay`
  (`|ExecutionSequence`
    (:`then_0`
      ; 입력 초기화
      (`EnhancedInputSubsystemInterface.AddMappingContext` (subsystem `EnhancedInputLocalPlayerSubsystem`) "/Game/Blueprints/Input/IMC_Game.IMC_Game" 0 (struct)))
    (:`then_1`
      ; HUD 초기화
      (`UserWidget.AddToViewport` (`self.HUD`) 0)
      (`self.UpdateShowDialogUI` (`self.IsShowDialog`)))
    (:`then_2`
      ; Cinematic 초기화
      (bind _outactors (`GameplayStatics.GetAllActorsOfClass` "/Game/Blueprints/Cinematic/BP_CinematicManager.BP_CinematicManager_C"))
      (set `self.CinematicManager` (`|GetArrayItem` _outactors)))))

(event `UpdateShowDialogUI`
  (params (IsShow :type Boolean))
  (bind _dialogpannel (`/Game/Blueprints/Cinematic/WBP_CinematicHUD.DialogPannel` (`self.HUD`)))
  ; 대화 보이기
  (bind _output_get (set `self.IsShowDialog` IsShow))
  (if _output_get
    (`Widget.SetVisibility` _dialogpannel "Visible")
    (else
      (`Widget.SetVisibility` _dialogpannel "Hidden"))))

(event `EnhancedInput|/Game/Blueprints/Input/Actions/IA_Space`
  (params (ActionValue :type Boolean) (ElapsedSeconds :type "Float (double-precision)") (TriggeredSeconds :type "Float (double-precision)") (InputAction :type "InputAction Object Reference" :default "/Game/Blueprints/Input/Actions/IA_Space.IA_Space"))
  (bind _output_scenes (break `/Game/Blueprints/Cinematic/ChapterData` (`|GetArrayItem` (`/Game/Blueprints/Cinematic/WBP_CinematicHUD.Chapters` (`self.HUD`)) (- (`self.ChapterStep`) 1))))
  (bind _output_dialogs (break `/Game/Blueprints/Cinematic/SceneData` (`|GetArrayItem` _output_scenes (- (`self.SceneStep`) 1))))
  ; 대화 넘기기 & 다음 씬 재생
  (:`Started`
    (if (`self.IsShowDialog`)
      (bind _result (`/Engine/EditorBlueprintResources/StandardMacros.IncrementInt` (`self.DialogStep`))
        (:`  `
          (if (< (- _result 1) (`KismetArrayLibrary.Array_Length` _output_dialogs))
            (`Image.SetBrush` (`/Game/Blueprints/Cinematic/WBP_CinematicHUD.Dialog` (`self.HUD`)) (make `SlateBrush` (struct :`SpecifiedColor` (struct :`R` 1.0 :`G` 1.0 :`B` 1.0 :`A` 1.0) :`ColorUseRule` "UseColor_Specified") "Image" "NoTile" "NoMirror" (struct :`X` 32.0 :`Y` 32.0) (struct) (`|GetArrayItem` _output_dialogs (- (`self.DialogStep`) 1))))
            (else
              (set `self.DialogStep` 0)
              (`/Engine/EditorBlueprintResources/StandardMacros.IncrementInt` (`self.SceneStep`)
                (:`  `
                  (`self.UpdateShowDialogUI` false)
                  (`/Game/Blueprints/Cinematic/BP_CinematicManager.PlayNextSquence` (`self.CinematicManager`)))))))))))

(fn `UserConstructionScript`)