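; BP_Battery is a turret that hunts the nearest actor tagged DamagableByBattery and fires beams at it.
; A Tick-driven state machine moves from Idle to Aim when a target is in range, computing a local look-at rotation and showing a laser after a brief delay.
; A sustained aim spawns BP_BatteryBeam, then cools down.
; The third hit breaks it, swapping the mesh, spawning effects and halting the cycle.
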(event `OnDamaged`
  ; 피격
  (bind _result (`/Engine/EditorBlueprintResources/StandardMacros.IncrementInt` (`self.DamagedCount`))
    (:`  `
      (if (== _result 3)
        (`self.OnBroken`)))))

(event `OnBroken`
  (bind _headcollision (`self.HeadCollision`))
  (bind _bodycollision (`self.BodyCollision`))
  ; 부숴지기
  (set `SkeletalMeshComponent.SkeletalMeshAsset` "/Game/Assets/Battery/BatteryBroken/BatteryBroken.BatteryBroken" (`self.SkeletalMesh`))
  (`GameplayStatics.SpawnEmitterAttached` "/Game/Realistic_Starter_VFX_Pack_Vol2/Particles/Smoke/P_Smoke_B.P_Smoke_B" _bodycollision "None" (0.0 0.0 0.0) (struct) (15.0 15.0 15.0))
  (`PrimitiveComponent.SetCollisionEnabled` _headcollision "NoCollision")
  (`GameplayStatics.SpawnEmitterAttached` "/Game/Realistic_Starter_VFX_Pack_Vol2/Particles/Sparks/P_Sparks_C.P_Sparks_C" _bodycollision "None" (0.0 0.0 0.0) (struct) (15.0 15.0 15.0))
  (`|SpawnActorFromClass` "/Game/Blueprints/Effect/BP_BatteryBrokenEffect.BP_BatteryBrokenEffect_C" (`KismetMathLibrary.MakeTransform` (`SceneComponent.K2_GetComponentLocation` _headcollision) (struct) (30.0 30.0 30.0)) "Undefined" "MultiplyWithRoot" null null)
  (`self.ChangeState` "NewEnumerator2"))

(event `ChangeState`
  (params (NextState :type "/Game/Blueprints/Battery/EBatteryState Enum" :default "NewEnumerator0"))
  ; 상태 전이
  (`|ExecutionSequence`
    (:`then_0`
      (switch `/Game/Blueprints/Battery/EBatteryState` (`self.CurrState`)
        (:`NewEnumerator1`
          (`SceneComponent.SetVisibility` (`self.AimLaser`) false false))))
    (:`then_1`
      (`|ExecutionSequence`
        (:`then_0`
          (switch `/Game/Blueprints/Battery/EBatteryState` NextState
            (:`NewEnumerator1`
              (set `self.AimingTime` 0.0))
            (:`NewEnumerator3`
              (set `self.AttackDelayTime` 0.0))))
        (:`then_1`
          (set `self.CurrState` NextState))))))

(event `self.ReceiveTick`
  (params (DeltaSeconds :type "Float (single-precision)"))
  (switch `/Game/Blueprints/Battery/EBatteryState` (`self.CurrState`)
    (:`NewEnumerator0`
      ; Idle -> Aim
      (set `self.MinDistance` 50000.0)
      (bind _outactors (`GameplayStatics.GetAllActorsWithTag` "DamagableByBattery"))
      (for _array_element _outactors
        (bind _returnvalue (`self.K2_GetActorLocation` _array_element))
        (bind _returnvalue_2 (`KismetMathLibrary.Vector_Distance` (`SceneComponent.K2_GetComponentLocation` (`self.HeadCollision`)) _returnvalue))
        (if (< _returnvalue_2 (`self.MinDistance`))
          (set `self.MinDistance` _returnvalue_2)
          (set `self.TargetLocation` (+ _returnvalue (0.0 0.0 40.0)))))
      (if (< (`self.MinDistance`) (`self.TraceRadius`))
        (`self.ChangeState` "NewEnumerator1")))
    (:`NewEnumerator1`
      (`|ExecutionSequence`
        (:`then_0`
          ; 타깃 조준하기
          (set `self.MinDistance` 50000.0)
          (bind _outactors_2 (`GameplayStatics.GetAllActorsWithTag` "DamagableByBattery"))
          (for _array_element_2 _outactors_2
            (bind _returnvalue_3 (`self.K2_GetActorLocation` _array_element_2))
            (bind _returnvalue_4 (`KismetMathLibrary.Vector_Distance` (`SceneComponent.K2_GetComponentLocation` (`self.HeadCollision`)) _returnvalue_3))
            (if (< _returnvalue_4 (`self.MinDistance`))
              (set `self.MinDistance` _returnvalue_4)
              (set `self.TargetLocation` (+ _returnvalue_3 (0.0 0.0 40.0)))))
          (if (< (`self.MinDistance`) (`self.TraceRadius`))
            (bind _output_get (set `self.LookAtDir` (`KismetMathLibrary.Normal` (- (`self.TargetLocation`) (`SceneComponent.K2_GetComponentLocation` (`self.HeadCollision`))))))
            (set `self.LookAtRot` (`KismetMathLibrary.MakeRotFromZ` (`KismetMathLibrary.Normal` (`KismetMathLibrary.InverseTransformDirection` (`self.GetTransform`) _output_get))))
            (else
              (`self.ChangeState` "NewEnumerator0"))))
        (:`then_1`
          ; 조준 레이저 이펙트
          (`NiagaraComponent.SetVariableVec3` (`self.AimLaser`) "Beam Start" (`SceneComponent.K2_GetComponentLocation` (`self.HeadCollision`)))
          (`NiagaraComponent.SetVariableVec3` (`self.AimLaser`) "Beam End" (`self.TargetLocation`))
          (if (> (`self.AimingTime`) 0.5)
            (`SceneComponent.SetVisibility` (`self.AimLaser`) true false)))
        (:`then_2`
          ; 조준 시간 재기 & 격발
          (bind _output_get_2 (set `self.AimingTime` (+ (`self.AimingTime`) DeltaSeconds)))
          (if (>= _output_get_2 5.0)
            (`self.Fire`)
            (`self.ChangeState` "NewEnumerator3")))))
    (:`NewEnumerator3`
      ; AttackDelay -> Idle
      (bind _output_get_3 (set `self.AttackDelayTime` (+ (`self.AttackDelayTime`) DeltaSeconds)))
      (if (>= _output_get_3 2.0)
        (`self.ChangeState` "NewEnumerator0")))))

(event `Fire`
  ; 빔 쏘기
  (bind _returnvalue (`|SpawnActorFromClass` "/Game/Blueprints/Effect/BP_BatteryBeam.BP_BatteryBeam_C" (`KismetMathLibrary.MakeTransform` (`self.K2_GetActorLocation`)) "Undefined" "MultiplyWithRoot" null null))
  (set `/Game/Blueprints/Effect/BP_BatteryBeam.OwnerBattery` self _returnvalue)
  (set `/Game/Blueprints/Effect/BP_BatteryBeam.TargetLoc` (`self.TargetLocation`) _returnvalue))

(fn `UserConstructionScript`)