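; BP_GanonBullet2 is a projectile, by its name fired by Ganon, that damages Link on impact.
; It faces along its velocity every tick, emits a tinted shockwave particle on its first tick and destroys itself after a timed lifetime.
; Collision hits, except on ArrowCollision-tagged components, damage actors tagged Link with a knock direction, spawn thunder-ball and explosion effects, then destroy the bullet.
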(event `self.ReceiveBeginPlay`
  (add `PrimitiveComponent.OnComponentHit` (`self.Collision`) (delegate `OnHit`))
  (`self.K2_SetActorRotation` (`KismetMathLibrary.MakeRotFromX` (`KismetMathLibrary.Normal` (`MovementComponent.Velocity` (`self.ProjectileMovement`))))))

(event `OnHit`
  (params (HitComponent :type "PrimitiveComponent Object Reference") (OtherActor :type "Actor Object Reference") (OtherComp :type "PrimitiveComponent Object Reference") (NormalImpulse :type "Vector Structure") (Hit :type "HitResult Structure (by ref)"))
  (if (not (`ActorComponent.ComponentHasTag` OtherComp "ArrowCollision"))
    (`|ExecutionSequence`
      (:`then_0`
        (if (`self.ActorHasTag` OtherActor "Link")
          (bind _asbp_link (cast `/Game/Blueprints/Link/BP_Link` OtherActor))
          (`/Game/Blueprints/Link/BP_Link.OnDamaged` _asbp_link (`KismetMathLibrary.Normal` (- (`self.K2_GetActorLocation` OtherActor) Hit_Location)))))
      (:`then_1`
        (`|SpawnActorFromClass` "/Game/FXVarietyPack/Blueprints/BP_ky_ThunderBallHit.BP_ky_ThunderBallHit_C" (`KismetMathLibrary.MakeTransform` Hit_Location (struct) (0.8 0.8 0.8)) "Undefined" "MultiplyWithRoot" null null)
        (`|SpawnActorFromClass` "/Game/Blueprints/Effect/BP_Explosion.BP_Explosion_C" (`KismetMathLibrary.MakeTransform` Hit_Location (struct) (1.5 1.5 1.5)) "Undefined" "MultiplyWithRoot" null null)
        (`self.K2_DestroyActor`)))))

(event `self.ReceiveTick`
  (params (DeltaSeconds :type "Float (single-precision)"))
  (bind (_returnvalue_location _returnvalue_rotation) (`KismetMathLibrary.BreakTransform` (`self.GetTransform`)))
  (`self.K2_SetActorRotation` (`KismetMathLibrary.MakeRotFromX` (`KismetMathLibrary.Normal` (`MovementComponent.Velocity` (`self.ProjectileMovement`)))))
  (`|ExecutionSequence`
    (:`then_0`
      (if (not (`self.HasSpawnEffect`))
        (bind _returnvalue (`GameplayStatics.SpawnEmitterAtLocation` "/Game/FXVarietyPack/Particles/P_ky_shotShockwave.P_ky_shotShockwave" _returnvalue_location _returnvalue_rotation (8.0 8.0 8.0)))
        (`ParticleSystemComponent.SetVectorParameter` _returnvalue "color" (3.0 2.7 0.33))
        (set `self.HasSpawnEffect` true)))
    (:`then_1`
      (bind _output_get (set `self.LifeTime` (+ (`self.LifeTime`) DeltaSeconds)))
      (if (>= _output_get 30.0)
        (`self.K2_DestroyActor`)))))

(fn `UserConstructionScript`)