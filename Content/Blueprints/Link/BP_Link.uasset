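; Player character Link, with third-person movement, jumping, paragliding with updrafts, and bow combat.
; A state machine (Locomotion, Glide, Draw, Aim, Disarm, Recoil) swaps movement settings, bow socket and reticle, with Tick running timed transitions.
; Drawing mid-air triggers slow motion, compensated on mesh animation and trail, while real-time deltas drive aim timers and camera zoom.
; Tick also computes hand IK targets and the aim direction used to launch spawned arrows.
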(event `SetTimeDilation`
  (params (TimeDilation :type "Float (double-precision)"))
  (bind _returnvalue (/ 1.0 TimeDilation))
  ; 시간 팽창
  (`GameplayStatics.SetGlobalTimeDilation` TimeDilation)
  (set `SkeletalMeshComponent.GlobalAnimRateScale` _returnvalue (`self.Mesh`))
  (`NiagaraComponent.SetCustomTimeDilation` (`self.TrailEffect`) _returnvalue))

(event `ChangeState`
  (params (NxtState :type "/Game/Blueprints/Link/ELinkState Enum" :default "NewEnumerator0"))
  ; 상태 전이
  (`|ExecutionSequence`
    (:`then_0`
      (switch `/Game/Blueprints/Link/ELinkState` (`self.CurState`)
        (:`NewEnumerator1`
          (`self.SetMovementLoco` :!label _label))
        (:`NewEnumerator2`
          (`|ExecutionSequence`
            (:`then_0`
              (goto _label))
            (:`then_1`
              (if (and (`|EnumInequality` NxtState "NewEnumerator3") (`self.CanDrawInput`))
                (`self.SetTimeDilation` 1.0)))))
        (:`NewEnumerator3`
          (if (`self.CanDrawInput`)
            (`self.SetTimeDilation` 1.0)
            (goto _label)))))
    (:`then_1`
      (bind _output_get (set `self.CurState` NxtState)))
    (:`then_2`
      (switch `/Game/Blueprints/Link/ELinkState` _output_get
        (:`NewEnumerator0`
          (`self.SetBowToBack` :!label _label_2))
        (:`NewEnumerator1`
          (goto _label_2))
        (:`NewEnumerator2`
          (bind _asbp_controller (cast `/Game/Blueprints/Game/BP_Controller` (`self.GetController`)))
          (`/Game/Blueprints/Game/BP_Controller.ShowAimingRecticle` _asbp_controller true)
          (`self.SetBowToHand`)
          (`self.SetMovementDrawAndAim` :!label _label_3))
        (:`NewEnumerator3`
          (goto _label_3))
        (:`NewEnumerator4`
          (`/Game/Blueprints/Game/BP_Controller.ShowAimingRecticle` _asbp_controller false :!label _label_4))
        (:`NewEnumerator5`
          (goto _label_4))))))

(event `self.ReceiveBeginPlay`
  ; Init
  (set `self.PrevUnpausedTime` (`GameplayStatics.GetRealTimeSeconds`))
  (bind _asbp_game_mode (cast `/Game/Blueprints/Game/BP_GameMode` (`GameplayStatics.GetGameMode`)))
  (switch `int` (`/Game/Blueprints/Game/BP_GameMode.Chapter` _asbp_game_mode)
    (:`1`
      (`self.SetActorActivate` false))))

(event `SetActorActivate`
  (params (IsActive :type Boolean))
  ; Activation
  (`self.SetActorHiddenInGame` (not IsActive))
  (`self.SetActorEnableCollision` IsActive)
  (`self.SetActorTickEnabled` IsActive)
  (`ActorComponent.SetActive` (`self.CharacterMovement`) IsActive false))

(event `EnhancedInput|/Game/Input/Actions/IA_Look`
  (params (ActionValue :type "Vector2D Structure") (ElapsedSeconds :type "Float (double-precision)") (TriggeredSeconds :type "Float (double-precision)") (InputAction :type "InputAction Object Reference" :default "/Game/Input/Actions/IA_Look.IA_Look"))
  ; 카메라 회전
  (:`Triggered`
    (`self.AddControllerYawInput` ActionValue_X)
    (`self.AddControllerPitchInput` (* ActionValue_Y -1.0))))

(event `EnhancedInput|/Game/Input/Actions/IA_Move`
  (params (ActionValue :type "Vector2D Structure") (ElapsedSeconds :type "Float (double-precision)") (TriggeredSeconds :type "Float (double-precision)") (InputAction :type "InputAction Object Reference" :default "/Game/Input/Actions/IA_Move.IA_Move"))
  (bind (_returnvalue_roll _returnvalue_pitch _returnvalue_yaw) (`KismetMathLibrary.BreakRotator` (`self.GetControlRotation`)))
  ; 이동
  (:`Triggered`
    (`self.AddMovementInput` (`KismetMathLibrary.GetRightVector` (`self.GetControlRotation`)) ActionValue_X)
    (`self.AddMovementInput` (`KismetMathLibrary.GetForwardVector` (`KismetMathLibrary.MakeRotator` 0.0 0.0 _returnvalue_yaw)) ActionValue_Y)))

(event `self.ReceiveTick`
  (params (DeltaSeconds :type "Float (single-precision)"))
  (bind _returnvalue (`GameplayStatics.GetRealTimeSeconds`))
  (bind _charactermovement (`self.CharacterMovement`))
  (bind _realdelta (`self.RealDelta`))
  (bind _realdelta_2 (`self.RealDelta`))
  (bind _glidefallspeed (`self.GlideFallSpeed`))
  (bind _curstate (`self.CurState`))
  (bind (_location _rotation) (`Controller.GetPlayerViewPoint` (`self.GetController`)))
  (bind (_velocity_x _velocity_y _velocity_z) (`KismetMathLibrary.BreakVector` (`MovementComponent.Velocity` (`self.CharacterMovement`))))
  (bind (_velocity_x_2 _velocity_y_2 _velocity_z_2) (`KismetMathLibrary.BreakVector` (`MovementComponent.Velocity` (`self.CharacterMovement`))))
  (set `self.RealDelta` (- _returnvalue (`self.PrevUnpausedTime`)))
  (set `self.PrevUnpausedTime` _returnvalue)
  (`|ExecutionSequence`
    (:`then_0`
      (switch `/Game/Blueprints/Link/ELinkState` (`self.CurState`)
        (:`NewEnumerator0`
          ; 떨어질 때 물리 세팅
          (if (`NavMovementComponent.IsFalling` _charactermovement)
            (set `CharacterMovementComponent.RotationRate` (struct :`Yaw` 20.0) _charactermovement)
            (else
              (set `CharacterMovementComponent.RotationRate` (struct :`Yaw` 360.0) _charactermovement))))
        (:`NewEnumerator1`
          ; Tick Glide
          (bind _asbp_game_mode (cast `/Game/Blueprints/Game/BP_GameMode` (`GameplayStatics.GetGameMode`)))
          (if (or (`self.IsInUpdraft`) (== (`/Game/Blueprints/Game/BP_GameMode.Chapter` _asbp_game_mode) 1))
            ;; 상승기류
            (set `MovementComponent.Velocity` (`KismetMathLibrary.MakeVector` _velocity_x_2 _velocity_y_2 (`KismetMathLibrary.FInterpTo` _velocity_z_2 (`self.TargetUpSpeed`) DeltaSeconds 10.0)) (`self.CharacterMovement`))
            (else
              ;; 글라이딩
              (if (< _velocity_z _glidefallspeed)
                (set `MovementComponent.Velocity` (`KismetMathLibrary.MakeVector` _velocity_x _velocity_y _glidefallspeed) (`self.CharacterMovement`))))))
        (:`NewEnumerator2`
          ; Tick Draw
          (`|ExecutionSequence`
            (:`then_0`
              (bind _output_get (set `self.DrawTime` (+ (`self.DrawTime`) _realdelta_2)))
              (if (>= _output_get 0.5)
                (`self.ChangeState` "NewEnumerator3")))
            (:`then_1`
              ;; 카메라 줌 당기기
              (set `self.CameraAimingTime` (`KismetMathLibrary.FClamp` (+ (`self.CameraAimingTime`) _realdelta_2) 0.0 0.5))
              (set `SpringArmComponent.SocketOffset` (`|EaseFunction` "EaseInOut" (`KismetMathLibrary.FClamp` (* (`self.CameraAimingTime`) 2.0)) (`KismetMathLibrary.Vector_Zero`) (150.0 75.0 30.0)) (`self.SpringArm`)))))
        (:`NewEnumerator4`
          ; Tick Disarm
          (bind _output_get_2 (set `self.DrawTime` (- (`self.DrawTime`) _realdelta)))
          (`|ExecutionSequence`
            (:`then_0`
              (if (<= _output_get_2 0.0)
                (`self.ChangeState` "NewEnumerator0")
                (`self.SetShowArrow` false)))))
        (:`NewEnumerator5`
          ; Tick Recoil
          (bind _output_get_3 (set `self.RecoilTime` (+ (`self.RecoilTime`) _realdelta)))
          (if (>= _output_get_3 0.5)
            (`self.ChangeState` "NewEnumerator4")))))
    (:`then_1`
      ; 조준 관련 값들 저장
      (bind _output_get_4 (set `self.AimPoint` (+ _location (* (`KismetMathLibrary.GetForwardVector` _rotation) (5000.0 5000.0 5000.0)))))
      (bind _output_get_5 (set `self.LeftHand` (`SceneComponent.GetSocketLocation` (`self.Mesh`) "Wrist_L")))
      (set `self.RightHand` (`SceneComponent.GetSocketLocation` (`self.Mesh`) "Wrist_R"))
      (set `self.AimDir` (`KismetMathLibrary.Normal` (- _output_get_4 _output_get_5)))
      (set `self.LeftHandIKTarget_CS` (`KismetMathLibrary.InverseTransformLocation` (`SceneComponent.K2_GetComponentToWorld` (`self.Mesh`)) (+ (`self.LeftHand`) (* (`self.AimDir`) (10000.0 10000.0 10000.0)))))
      (set `self.RightHandIKTarget_CS` (`KismetMathLibrary.InverseTransformLocation` (`SceneComponent.K2_GetComponentToWorld` (`self.Mesh`)) (+ (`self.RightHand`) (* (`KismetMathLibrary.Normal` (- (`self.AimPoint`) (`self.RightHand`))) (10000.0 10000.0 10000.0))))))
    (:`then_2`
      ; 카메라 줌 아웃
      (if (and (`|EnumInequality` _curstate "NewEnumerator2") (`|EnumInequality` _curstate "NewEnumerator3"))
        (set `self.CameraAimingTime` (`KismetMathLibrary.FClamp` (- (`self.CameraAimingTime`) _realdelta) 0.0 0.5))
        (set `SpringArmComponent.SocketOffset` (`|EaseFunction` "EaseInOut" (`KismetMathLibrary.FClamp` (* (`self.CameraAimingTime`) 2.0)) (`KismetMathLibrary.Vector_Zero`) (150.0 75.0 30.0)) (`self.SpringArm`))))))

(event `EnhancedInput|/Game/Input/Actions/IA_JumpAndGlide`
  (params (ActionValue :type Boolean) (ElapsedSeconds :type "Float (double-precision)") (TriggeredSeconds :type "Float (double-precision)") (InputAction :type "InputAction Object Reference" :default "/Game/Input/Actions/IA_JumpAndGlide.IA_JumpAndGlide"))
  ; 점프
  (:`Started`
    (bind _asbp_controller (cast `/Game/Blueprints/Game/BP_Controller` (`self.GetController`)))
    (if (not (`Widget.IsVisible` (`/Game/Blueprints/UI/WBP_HUD.TitlePanel` (`/Game/Blueprints/Game/BP_Controller.HUD` _asbp_controller))))
      (switch `/Game/Blueprints/Link/ELinkState` (`self.CurState`)
        (:`NewEnumerator0`
          (if (not (`NavMovementInterface.IsFalling` (`self.CharacterMovement`))) :!label _label_5
            (`self.Jump`)
            (else
              (`self.Glide`))))
        (:`NewEnumerator1`
          (`self.ChangeState` "NewEnumerator0"))
        (:`NewEnumerator4`
          (`self.SetShowArrow` false)
          (goto _label_5))
        (:`NewEnumerator5`
          (goto _label_5))))))

(event `SetMovementDrawAndAim`
  (bind _charactermovement (`self.CharacterMovement`))
  ; 조준 움직임 세팅
  (set `CharacterMovementComponent.MaxWalkSpeed` 300.0 _charactermovement)
  (set `CharacterMovementComponent.bOrientRotationToMovement` false _charactermovement)
  (set `self.bUseControllerRotationYaw` true))

(event `SetMovementLoco`
  (bind _charactermovement (`self.CharacterMovement`))
  ; 기본 움직임 세팅
  (set `CharacterMovementComponent.GravityScale` 1.0 _charactermovement)
  (set `CharacterMovementComponent.AirControl` 0.05 _charactermovement)
  (set `CharacterMovementComponent.BrakingDecelerationFalling` 0.0 _charactermovement)
  (set `CharacterMovementComponent.FallingLateralFriction` 0.0 _charactermovement)
  (set `CharacterMovementComponent.RotationRate` (struct :`Yaw` 360.0) _charactermovement)
  (set `CharacterMovementComponent.MaxWalkSpeed` 600.0 _charactermovement)
  (set `CharacterMovementComponent.bOrientRotationToMovement` true _charactermovement)
  (set `self.bUseControllerRotationYaw` false)
  (`SceneComponent.SetVisibility` (`self.Paraglider`) false false))

(event `self.OnLanded`
  (params (Hit :type "HitResult Structure (by ref)"))
  ; OnLanded
  (switch `/Game/Blueprints/Link/ELinkState` (`self.CurState`)
    (:`NewEnumerator1`
      (`self.ChangeState` "NewEnumerator0"))
    (:`NewEnumerator2`
      (`self.SetTimeDilation` 1.0 :!label _label_6))
    (:`NewEnumerator3`
      (goto _label_6))))

(event `SetBowToHand`
  ; 활, 화살 메시 업데이트
  (`SceneComponent.K2_AttachToComponent` (`self.Bow`) (`self.Mesh`) "WeaponBow" "KeepRelative" "KeepRelative" "KeepRelative" true))

(event `SetBowToBack`
  ; 활, 화살 메시 업데이트
  (`SceneComponent.K2_AttachToComponent` (`self.Bow`) (`self.Mesh`) "BackBow" "KeepRelative" "KeepRelative" "KeepRelative" true))

(event `SetShowArrow`
  (params (IsShow :type Boolean))
  (bind _weaponarrow (`self.WeaponArrow`))
  ; 활, 화살 메시 업데이트
  (`SceneComponent.SetVisibility` _weaponarrow IsShow true)
  (`SceneComponent.SetHiddenInGame` _weaponarrow (not IsShow) true))

(event `EnhancedInput|/Game/Input/Actions/IA_DrawAndAim`
  (params (ActionValue :type Boolean) (ElapsedSeconds :type "Float (double-precision)") (TriggeredSeconds :type "Float (double-precision)") (InputAction :type "InputAction Object Reference" :default "/Game/Input/Actions/IA_DrawAndAim.IA_DrawAndAim"))
  ; 활 조준 입력
  (:`Started`
    (if (`self.CanDrawInput`)
      (switch `/Game/Blueprints/Link/ELinkState` (`self.CurState`)
        (:`NewEnumerator0`
          _)
        (:`NewEnumerator1`
          _)
        (:`NewEnumerator4`
          _)
        (:`NewEnumerator5`
          _))
      (`self.ChangeState` "NewEnumerator2")
      (`self.SetShowArrow` true)
      (set `self.DrawTime` 0.0)
      (if (`NavMovementComponent.IsFalling` (`self.CharacterMovement`))
        (`self.SetTimeDilation` 0.05))))
  (:`Completed`
    (switch `/Game/Blueprints/Link/ELinkState` (`self.CurState`)
      (:`NewEnumerator2`
        _)
      (:`NewEnumerator3`
        _))
    (`self.ChangeState` "NewEnumerator4")))

(event `EnhancedInput|/Game/Input/Actions/IA_Shoot`
  (params (ActionValue :type Boolean) (ElapsedSeconds :type "Float (double-precision)") (TriggeredSeconds :type "Float (double-precision)") (InputAction :type "InputAction Object Reference" :default "/Game/Input/Actions/IA_Shoot.IA_Shoot"))
  ; 화살 발사 입력
  (:`Started`
    (if (`|EnumEquality` (`self.CurState`) "NewEnumerator3")
      (`self.ChangeState` "NewEnumerator5")
      (`self.SetShowArrow` false)
      (set `self.RecoilTime` 0.0)
      (bind _returnvalue (`|SpawnActorFromClass` "/Game/Blueprints/Projectile/BP_Arrow.BP_Arrow_C" (`KismetMathLibrary.MakeTransform` (`SceneComponent.GetSocketLocation` (`self.WeaponArrow`) "WeaponArrow")) "Undefined" "MultiplyWithRoot" null null))
      (bind _projectilemovement (`/Game/Blueprints/Projectile/BP_Arrow.ProjectileMovement` _returnvalue))
      (bind _initialspeed (`ProjectileMovementComponent.InitialSpeed` _projectilemovement))
      (set `MovementComponent.Velocity` (* (`self.AimDir`) (`KismetMathLibrary.MakeVector` _initialspeed _initialspeed _initialspeed)) _projectilemovement))))

(event `OnDamaged`
  (params (DamageDir :type "Vector Structure"))
  (`self.LaunchCharacter` (`KismetMathLibrary.MakeVector` (* DamageDir_X 500.0) (* DamageDir_Y 500.0) 700.0)))

(fn `Glide`
  (bind _charactermovement (`self.CharacterMovement`))
  (`self.ChangeState` "NewEnumerator1")
  ; 글라이딩 움직임 세팅
  (set `CharacterMovementComponent.GravityScale` 0.25 _charactermovement)
  (set `CharacterMovementComponent.AirControl` 0.8 _charactermovement)
  (set `CharacterMovementComponent.BrakingDecelerationFalling` 200.0 _charactermovement)
  (set `CharacterMovementComponent.FallingLateralFriction` 0.2 _charactermovement)
  (set `CharacterMovementComponent.RotationRate` (struct :`Yaw` 20.0) _charactermovement)
  (set `CharacterMovementComponent.MaxWalkSpeed` 1000.0 _charactermovement)
  (`SceneComponent.SetVisibility` (`self.Paraglider`) true false))

(fn `UserConstructionScript`)